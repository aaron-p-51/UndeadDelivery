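; BP_BrainPackage is a thrown brain projectile that is delivered to a target zombie.
; With a valid target, it caches the BrainTargetSocket location on BeginPlay and moves there at constant speed on Tick.
; Within a squared-distance threshold, it attaches to the socket, calls the zombie's OnReceivedBrain and stops ticking.
; Without a target, it simulates physics, gets a push based on its Y position and expires after a short lifespan.
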(event Custom|MoveToTargetZombie
  (params (DeltaSeconds :type Float%20%28single-precision%29))
  (Transformation|SetActorLocation (Math|Interpolation|VInterptoConstant (Transformation|GetActorLocation) (Variables|State|GetTargetLocation) DeltaSeconds (Variables|Gameplay|GetThrowToZombieSpeed)) false false))

(event EventBeginPlay
  (bind _zombietarget (Variables|State|GetZombieTarget))
  (bind _sphere (Variables|Default|GetSphere))
  (Utilities|IsValid _zombietarget
    (:Is%20Valid
      (Variables|State|SetTargetLocation (Transformation|GetSocketLocation (Variables|/Game/Game/Blueprints/BP_Zombie.BP_Zombie_C|GetSkeletalMesh _zombietarget) "BrainTargetSocket"))
      (Variables|State|SetHasTarget true))
    (:Is%20Not%20Valid
      (Physics|SetSimulatePhysics (Variables|Default|GetSphere) true)
      (if (> (.y (Transformation|GetActorLocation)) 0.0)
        (Physics|AddForce _sphere "0,1000.000000, 0" "None" false)
        (else
          (Physics|AddForce _sphere (Math|Vector|RotateVector (Variables|Gameplay|GetThrowNoZombieForce) "180.000000, 0, 0") "None" false)))
      (Actor|SetLifeSpan 1.0))))

(event EventTick
  (params (DeltaSeconds :type Float%20%28single-precision%29))
  (bind _zombietarget (Variables|State|GetZombieTarget))
  (if (Variables|State|GetHasTarget)
    (CallFunction|MovetoTargetZombie DeltaSeconds)
    (bind _result (CallFunction|IsWithinTargetDistanceThreshold))
    (if _result
      (Transformation|AttachComponentToComponent (Variables|/Game/Game/Blueprints/BP_Zombie.BP_Zombie_C|GetSkeletalMesh _zombietarget) "BrainTargetSocket" "KeepWorld" "KeepWorld" "KeepWorld" false)
      (Default|OnReceivedBrain _zombietarget self)
      (Actor|Tick|SetActorTickEnabled false))))

(fn ConstructionScript)

(fn IsWithinTargetDistanceThreshold
  (return (< (Class|KismetMathLibrary|VectorDistanceSquared (Transformation|GetActorLocation) (Variables|State|GetTargetLocation)) (Variables|Gameplay|GetDistanceToTargetThreshold))))