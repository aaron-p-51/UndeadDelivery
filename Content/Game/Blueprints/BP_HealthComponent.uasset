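; Health component that tracks an owner's health and grants temporary invincibility after each hit.
; BeginPlay sets current health to the default; LoseHealth removes one point, ignoring its Amount input, clamps at zero and broadcasts the new value.
; A timer ends the invincibility window, with dispatchers announcing both state changes.
; LoseHealth also compares game time against LastTimeHealthLost, which this graph never updates.
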(event Custom|LoseHealth
  (params (Amount :type Integer))
  (if (and (not (Variables|State|GetInvincibleAfterHealthLoss)) (>= (Utilities|Time|GetTimeSeconds) (+ (Variables|State|GetLastTimeHealthLost) (Variables|GamePlay|GetHealthLossInvincibilityTime))))
    (if (!= (Variables|State|GetCurrentHealth) (Math|Integer|Max(Integer) 0 (- (Variables|State|GetCurrentHealth) 1)))
      (bind _output_get (Variables|State|SetCurrentHealth (Math|Integer|Max(Integer) 0 (- (Variables|State|GetCurrentHealth) 1))))
      (Default|CallOnHealthValueChanged _output_get)
      (bind _output_get_2 (Variables|State|SetInvincibleAfterHealthLoss true))
      (Default|CallInvincibilityChange _output_get_2)
      (Utilities|Time|SetTimerbyEvent (delegate Custom|EndInvincibility) (Variables|GamePlay|GetHealthLossInvincibilityTime)))))

(event Custom|EndInvincibility
  (bind _output_get (Variables|State|SetInvincibleAfterHealthLoss false))
  (Default|CallInvincibilityChange _output_get))

(event EventBeginPlay
  (Variables|State|SetCurrentHealth (Variables|GamePlay|GetDefaultHealth)))

(event EventTick
  (params (DeltaSeconds :type Float%20%28single-precision%29)))