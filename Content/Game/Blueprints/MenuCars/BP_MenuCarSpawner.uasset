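; BP_MenuCarSpawner periodically spawns random obstacle cars, flagged as menu cars, at its own transform.
; BeginPlay schedules the first spawn at a random delay within a min/max range.
; Tick compares game time to that scheduled time, then spawns a random class from the ObstacleCars array with a fixed forward speed and schedules the next spawn.
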(event Custom|SetNextSpawnTime
  (Variables|Default|SetNextSpawnTime (+ (Utilities|Time|GetTimeSeconds) (Math|Random|RandomFloatinRange (Variables|Default|GetMinSpawnDelay) (Variables|Default|GetMaxSpawnDelay)))))

(event EventBeginPlay
  (CallFunction|SetNextSpawnTime))

(event Collision|EventActorBeginOverlap
  (params (OtherActor :type Actor%20Object%20Reference)))

(event EventTick
  (params (DeltaSeconds :type Float%20%28single-precision%29))
  (bind _obstaclecars (Variables|Default|GetObstacleCars))
  (if (> (Utilities|Time|GetGameTimeinSeconds) (Variables|Default|GetNextSpawnTime))
    (Game|SpawnActorfromClass (Utilities|Array|Get(acopy) _obstaclecars (Math|Random|RandomIntegerinRange 0 (- (Utilities|Array|Length _obstaclecars) 1))) (Transformation|GetWorldTransform (Variables|Default|GetDefaultSceneRoot)) "Undefined" 0 1e+03 true 0)
    (CallFunction|SetNextSpawnTime)))

(fn ConstructionScript)