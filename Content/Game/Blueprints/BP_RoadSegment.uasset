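; Road segment for an endless road that dresses itself with random side houses and provides an attach point for the next segment.
; BeginPlay picks the houses and shows or hides a debug segment label based on the game mode.
; Separate events, not called on BeginPlay, spawn config-driven brain drop zones and random obstacle cars at marker components.
; Player overlap at the end trigger requests a new segment unless warmup, and the segment destroys itself after a delay.
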(event OnComponentBeginOverlap(EndOfRoadSegment)
  (params (OverlappedComponent :type Primitive%20Component%20Object%20Reference) (OtherActor :type Actor%20Object%20Reference) (OtherComp :type Primitive%20Component%20Object%20Reference) (OtherBodyIndex :type Integer) (bFromSweep :type Boolean) (SweepResult :type Hit%20Result%20Structure%20%28by%20ref%29))
  (bind _endlessconfigspawner (Variables|State|GetEndlessConfigSpawner))
  ;[1 1 1] Reached end of segment
  (Utilities|Casting|CastToBP_PlayerPawn OtherActor
    (:then
      ;;[1 1 1] Road Spawn System, spawn next segment
      (if (not (Variables|State|GetIsWarmupRoad))
        (Utilities|IsValid _endlessconfigspawner
          (:Is%20Valid
            (Default|NewSpawnRoadSegment _endlessconfigspawner))
          (:Is%20Not%20Valid
            _))))
    (:CastFailed
      _))
  ;;[1 1 1] Destroy this road segment
  (Utilities|FlowControl|Delay (Variables|Gameplay|GetDestroyDelay))
  (Actor|DestroyActor))

(event Custom|SpawnSideHouses
  ;[1 1 1] Spawn Left House Mesh
  (bind _house (CallFunction|GetRandomHouse))
  (Components|StaticMesh|SetStaticMesh (Variables|Default|GetLeftHouseMesh) _house)
  ;[1 1 1] Spawn Right House Mesh
  (bind _house_2 (CallFunction|GetRandomHouse))
  (Components|StaticMesh|SetStaticMesh (Variables|Default|GetRightHouseMesh) _house_2))

(event Custom|SetDebugRoadSegment
  (bind _debugroadsegmentnumber (Variables|Default|GetDebugRoadSegmentNumber))
  ;[1 1 1] Debug Road Segment Number
  (if (Variables|State|GetIsWarmupRoad)
    (Rendering|Components|TextRender|SetText _debugroadsegmentnumber (Utilities|Text|ToText(String) "W"))
    (else
      (Rendering|Components|TextRender|SetText _debugroadsegmentnumber (Utilities|Text|ToText(Integer) (Variables|State|GetRoadSegmentNumber))))))

(event Custom|SetBrainDeliveryPoints
  (switch Utilities|FlowControl|Switch|SwitchonEBP_BrainDelivery (.braindelivery (Variables|State|GetRoadSegmentConfig))
    (:NewEnumerator1
      (Game|SpawnActorfromClass "/Game/Game/Blueprints/BP_BrainDropZone.BP_BrainDropZone_C" (Transformation|GetWorldTransform (Variables|Default|GetLeftDropPoint)) "Undefined" 0 "NewEnumerator1" 0))
    (:NewEnumerator2
      (Game|SpawnActorfromClass "/Game/Game/Blueprints/BP_BrainDropZone.BP_BrainDropZone_C" (Transformation|GetWorldTransform (Variables|Default|GetRightDropPoint)) "Undefined" 0 "NewEnumerator2" 0))))

(event Custom|RemoveDebugSegmentVisibility
  ;[1 1 1] Debug Road Segment Number
  (Rendering|SetVisibility (Variables|Default|GetDebugRoadSegmentNumber) false false))

(event Custom|SetDebugTextRender
  ;[1 1 1] Debug Road Segment Number
  (bind _asbp_game_mode (Utilities|Casting|CastToBP_GameMode (Game|GetGameMode)))
  (bind _debugmode (Default|GetIsDebugMode _asbp_game_mode))
  (if _debugmode
    (CallFunction|SetDebugRoadSegment)
    (else
      (CallFunction|RemoveDebugSegmentVisibility))))

(event Custom|SpawnObstacleVehicles
  (bind _spawnableobsticalcars (Variables|Gameplay|GetSpawnableObsticalCars))
  (bind _asbp_game_mode (Utilities|Casting|CastToBP_GameMode (Game|GetGameMode)))
  (bind _speed (Default|GetObstacleCarSpeed _asbp_game_mode))
  (for _array_element (.vehiclespawns (Variables|State|GetRoadSegmentConfig))
    (if (Utilities|Enum|NotEqual(Enum) _array_element "NewEnumerator0")
      (bind _spawntransform (CallFunction|GetObstacleVehicleSpawnTransform _array_element))
      (Game|SpawnActorfromClass (Utilities|Array|Get(acopy) _spawnableobsticalcars (Math|Random|RandomIntegerinRange 0 (- (Utilities|Array|Length _spawnableobsticalcars) 1))) _spawntransform "AlwaysSpawn" 0 _speed 0))))

(event EventBeginPlay
  (CallFunction|SpawnSideHouses)
  (CallFunction|SetDebugTextRender)
  (if (not (Variables|State|GetIsWarmupRoad))
    _))

(fn ConstructionScript)

(fn GetNextSegmentAttachPoint
  (return (Transformation|GetWorldTransform (Variables|Default|GetNextSegmentAttachPoint))))

(fn GetRandomHouse
  (bind _spawnablesidehouse (Variables|Gameplay|GetSpawnableSideHouse))
  (return (Utilities|Array|Get(acopy) _spawnablesidehouse (Math|Random|RandomIntegerinRange 0 (- (Utilities|Array|Length _spawnablesidehouse) 1)))))

(fn GetObstacleVehicleSpawnTransform
  (params (SpawnSubSection :type EBP_ObstacleVehicleSpawnSubSection%20Enum :default "NewEnumerator0"))
  (switch Utilities|FlowControl|Switch|SwitchonEBP_ObstacleVehicleSpawnSubSection SpawnSubSection
    (:NewEnumerator0
      (return ""))
    (:NewEnumerator1
      (return (Transformation|GetWorldTransform (Variables|Default|GetObstacleVehicleSpawn_TL))))
    (:NewEnumerator2
      (return (Transformation|GetWorldTransform (Variables|Default|GetObstacleVehicleSpawn_TM))))
    (:NewEnumerator3
      (return (Transformation|GetWorldTransform (Variables|Default|GetObstacleVehicleSpawn_TR))))
    (:NewEnumerator5
      (return (Transformation|GetWorldTransform (Variables|Default|GetObstacleVehicleSpawn_BL))))
    (:NewEnumerator4
      (return (Transformation|GetWorldTransform (Variables|Default|GetObstacleVehicleSpawn_BM))))
    (:NewEnumerator6
      (return (Transformation|GetWorldTransform (Variables|Default|GetObstacleVehicleSpawn_BR))))))

(fn GetBrainDeliveryTransform
  (params (BrainDelivery :type EBP_BrainDelivery%20Enum :default "NewEnumerator0"))
  (switch Utilities|FlowControl|Switch|SwitchonEBP_BrainDelivery BrainDelivery
    (:NewEnumerator0
      (return ""))
    (:NewEnumerator1
      (return (Transformation|GetWorldTransform (Variables|Default|GetLeftDropPoint))))
    (:NewEnumerator2
      (return (Transformation|GetWorldTransform (Variables|Default|GetRightDropPoint))))))