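; Player vehicle pawn that auto-drives forward, steers within lane limits and throws brain packages at zombies in drop zones.
; Tick moves it using the brake component's state, then derives mesh tilt, spring arm length and engine audio from speed and turning, with tire screech on turns or braking.
; Throws are rate-limited and spawn from the socket on the pawn's current side.
; Hitting obstacle cars destroys them and costs health; invincibility flashes the mesh.
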(event OnComponentBeginOverlap(CollisionComp)
  (params (OverlappedComponent :type Primitive%20Component%20Object%20Reference) (OtherActor :type Actor%20Object%20Reference) (OtherComp :type Primitive%20Component%20Object%20Reference) (OtherBodyIndex :type Integer) (bFromSweep :type Boolean) (SweepResult :type Hit%20Result%20Structure%20%28by%20ref%29))
  ;[1 1 1] Bound Events
  ;;[1 1 1] Lose health
  (bind _asbp_obstacle_car_base (Utilities|Casting|CastToBP_ObstacleCarBase OtherActor))
  (Actor|DestroyActor _asbp_obstacle_car_base)
  (Default|LoseHealth (Variables|Default|GetBP_HealthComponent) (Variables|Gameplay|GetHealthLossFromObstacleHit)))

(event Custom|MoveForward
  (params (DeltaSeconds :type Float%20%28single-precision%29))
  ;[1 1 1] Move forward
  (bind _isbraking (Default|IsBraking (Variables|Default|GetBP_BrakeComponent)))
  (if _isbraking
    ;;[1 1 1] Braking
    (Variables|State|SetCurrentSpeed (Math|Interpolation|FInterptoConstant (Variables|State|GetCurrentSpeed) (Variables|Gameplay|Braking|GetForwardSpeedWhenBraking) DeltaSeconds (Variables|Gameplay|Braking|GetForwardSpeedToBrakeSpeedRate)))
    (else
      ;;[1 1 1] Not Braking
      (Variables|State|SetCurrentSpeed (Math|Interpolation|FInterptoConstant (Variables|State|GetCurrentSpeed) (Variables|Gameplay|GetForwardSpeed) DeltaSeconds (Variables|Gameplay|Braking|GetBrakeSpeedToForwardSpeedRate)))))
  (CallFunction|ComputeIsSlowingDown)
  (Transformation|SetActorLocation (+ (Transformation|GetActorLocation) (* (Transformation|GetActorForwardVector) (* (Variables|State|GetCurrentSpeed) DeltaSeconds))) false false))

(event Custom|TryDropBrainPackage
  (bind _collisioncomp (Variables|Default|GetCollisionComp))
  (bind _overlappingactors (Collision|GetOverlappingActors _collisioncomp "/Game/Game/Blueprints/BP_BrainDropZone.BP_BrainDropZone_C" :!class /Script/Engine.PrimitiveComponent))
  ;[1 1 1] Player Input
  ;;[1 1 1] Throw Brain
  (bind _result (CallFunction|EnoughTimeBetweenDrops))
  (if _result
    (if (> (Utilities|Array|Length _overlappingactors) 0)
      (bind _asbp_brain_drop_zone (Utilities|Casting|CastToBP_BrainDropZone (Utilities|Array|Get(acopy) _overlappingactors))
        (:then
          (Variables|/Game/Game/Blueprints/BP_BrainDropZone.BP_BrainDropZone_C|SetBrainDropedInZone _asbp_brain_drop_zone true)
          (bind _zombie (Default|GetZombie _asbp_brain_drop_zone))
          (Variables|State|SetZombieInCurrentDropZone _zombie))
        (:CastFailed
          (Variables|State|SetZombieInCurrentDropZone 0 :!label _label)))
      (else
        (goto _label)))
    (if (>= (.y (Transformation|GetWorldLocation (Variables|Default|GetVehicleRoot))) 0.0)
      (Game|SpawnActorfromClass "/Game/Game/Blueprints/BP_BrainPackage.BP_BrainPackage_C" (Transformation|GetSocketTransform (Variables|Default|GetVehicleStaticMesh) "RightPackageThrowPoint" "RTS_World") "Undefined" 0 (Variables|State|GetZombieInCurrentDropZone) 0)
      (else
        (Game|SpawnActorfromClass "/Game/Game/Blueprints/BP_BrainPackage.BP_BrainPackage_C" (Transformation|GetSocketTransform (Variables|Default|GetVehicleStaticMesh) "LeftPackageThrowPoint" "RTS_World") "Undefined" 0 (Variables|State|GetZombieInCurrentDropZone) 0)))
    (Audio|PlaySoundatLocation "/Game/Game/Audio/Cues/Cue_ThrowBrain.Cue_ThrowBrain" (Transformation|GetWorldLocation (Variables|Default|GetVehicleStaticMesh)) "0, 0, 0" 1.0 1.0 0.0 0 0 0)))

(event Custom|SetVehicleRotationVisuals
  (params (DeltaSeconds :type Float%20%28single-precision%29))
  (bind _vehicleroot (Variables|Default|GetVehicleRoot))
  (bind _vehiclestaticmesh (Variables|Default|GetVehicleStaticMesh))
  (bind _returnvalue (Transformation|GetWorldLocation _vehicleroot))
  ;[1 1 1] Vehicle yaw and roll movement
  (Transformation|SetRelativeRotation _vehiclestaticmesh (Math|Interpolation|RInterpTo (Variables|/Script/Engine.SceneComponent|GetRelativeRotation _vehiclestaticmesh) (Math|Rotator|MakeRotator (* (.roll (Math|Rotator|MakeRotator (* (- (Variables|State|GetPreviousTurnMovement) (.y _returnvalue)) (Variables|Gameplay|Visuals|GetRollTurnScale) -1.0) 0.0 (* (- (Variables|State|GetPreviousTurnMovement) (.y _returnvalue)) (Variables|Gameplay|Visuals|GetRollTurnScale) -1.0))) (Variables|Gameplay|Visuals|GetRollTurnScale)) (Math|Float|MapRangeClamped (Variables|State|GetCurrentSpeed) (Variables|Gameplay|GetForwardSpeed) (Variables|Gameplay|Braking|GetForwardSpeedWhenBraking) (Variables|Gameplay|Visuals|GetPitchAngleFullSpeed) (Variables|Gameplay|Visuals|GetPitchAngleBraking)) (* (.yaw (Math|Rotator|MakeRotator (* (- (Variables|State|GetPreviousTurnMovement) (.y _returnvalue)) (Variables|Gameplay|Visuals|GetRollTurnScale) -1.0) 0.0 (* (- (Variables|State|GetPreviousTurnMovement) (.y _returnvalue)) (Variables|Gameplay|Visuals|GetRollTurnScale) -1.0))) (Variables|Gameplay|Visuals|GetYawTurnScale))) DeltaSeconds (Variables|Gameplay|Visuals|GetBankTurnSmoothSpeed)) false false)
  (Variables|State|SetPreviousTurnMovement (.y _returnvalue)))

(event Custom|SetPlayerView
  ;[1 1 1] Visuals
  ;;[1 1 1] Set camera string arm target length based on forward speed, forward speed changes when braking
  (Variables|/Script/Engine.SpringArmComponent|SetTargetArmLength (Variables|Default|GetSpringArm) (Math|Float|MapRangeClamped (Variables|State|GetCurrentSpeed) (Variables|Gameplay|GetForwardSpeed) (Variables|Gameplay|Braking|GetForwardSpeedWhenBraking) (Variables|State|GetDefaultSprintArmLength) (Variables|Gameplay|Braking|GetBrakingSpringArmLength))))

(event Custom|OnHealthCompInvincibilityChange
  (params (Invincible :type Boolean))
  ;[1 1 1] Bind to HealthComponent events
  (CallFunction|HandleonHealthCompInvincibilityChange Invincible))

(event Custom|HandleOnHealthCompInvincibilityChange
  (params (Invincible :type Boolean))
  ;[1 1 1] Bound Events
  (Variables|State|SetFlashInvincibility Invincible))

(event Custom|FlashMesh
  ;[1 1 1] Visuals
  ;;[1 1 1] Not the ideal way to handle flashing mesh
  (if (> (Math|Trig|Sin(Radians) (* (Utilities|Time|GetTimeSeconds) (Variables|Gameplay|Visuals|GetInvincibilityFlashRate))) 0.0)
    (Rendering|SetVisibility (Variables|Default|GetVehicleStaticMesh) false false)
    (else
      (Rendering|SetVisibility (Variables|Default|GetVehicleStaticMesh) true false))))

(event Custom|SetPlayerVisibility
  ;[1 1 1] Visuals
  ;;[1 1 1] Set vehicle mesh visibility based on invincibility (Health Component)
  (if (Variables|State|GetFlashInvincibility)
    (CallFunction|FlashMesh)
    (else
      (Rendering|SetVisibility (Variables|Default|GetVehicleStaticMesh) true false))))

(event Custom|SetVehicleEngineAudioParams
  (Audio|Parameter|SetFloatParameter (Variables|Default|GetVehicleEngine) "ForwardSpeed" (Variables|State|GetCurrentSpeed) :!class /Script/Engine.AudioComponent)
  (CallFunction|PlayerTireScreechSound))

(event Custom|PlayerTireScreechSound
  (if (or (Variables|State|GetIsTurning) (Variables|State|GetIsSlowingDown))
    (Utilities|IsValid (Variables|State|GetTiresScreechSound)
      (:Is%20Not%20Valid
        (bind _returnvalue (Audio|SpawnSoundAttached "/Game/Game/Audio/Cues/Cue_PlayerCarTurnAndBrake.Cue_PlayerCarTurnAndBrake" (Variables|Default|GetVehicleStaticMesh) "None" "0, 0, 0" "0, 0, 0" "KeepRelativeOffset" false 1.0 1.0 0.0 0 0))
        (Variables|State|SetTiresScreechSound _returnvalue)))
    (else
      (Utilities|IsValid (Variables|State|GetTiresScreechSound)
        (:Is%20Valid
          (Audio|Components|Audio|StopDelayed (Variables|State|GetTiresScreechSound) 0.2)
          (Variables|State|SetTiresScreechSound 0))))))

(event EventBeginPlay
  (Utilities|FlowControl|Sequence
    (:then_0
      ;[1 1 1] Set initial variable values
      (Variables|State|SetCurrentSpeed (Variables|Gameplay|GetForwardSpeed))
      (Variables|State|SetDefaultSprintArmLength (Variables|/Script/Engine.SpringArmComponent|GetTargetArmLength (Variables|Default|GetSpringArm))))
    (:then_1
      ;[1 1 1] Bind to HealthComponent events
      (EventDispatchers|BindEventtoInvincibilityChange (Variables|Default|GetBP_HealthComponent) (delegate Custom|OnHealthCompInvincibilityChange)))))

(event EventTick
  (params (DeltaSeconds :type Float%20%28single-precision%29))
  (if (Variables|State|GetCanMove)
    (CallFunction|MoveForward DeltaSeconds)
    (CallFunction|SetVehicleRotationVisuals DeltaSeconds)
    (CallFunction|SetPlayerView)
    (CallFunction|SetPlayerVisibility)
    (CallFunction|SetVehicleEngineAudioParams)))

(event Input|ActionEvents|InputActionDropPackage
  (params (Key :type Key%20Structure :default "None"))
  ;[1 1 1] Player Input
  ;;[1 1 1] Drop brain package
  (:Pressed
    (CallFunction|TryDropBrainPackage)))

(event Input|ActionEvents|InputActionBrake
  (params (Key :type Key%20Structure :default "None"))
  (bind _bp_brakecomponent (Variables|Default|GetBP_BrakeComponent))
  ;[1 1 1] Player Input
  ;;[1 1 1] Apply/Release Brake
  (:Pressed
    (Default|StartUseBrake _bp_brakecomponent)
    (Variables|State|SetIsBraking true))
  (:Released
    (Default|StopUseBrake _bp_brakecomponent)
    (Variables|State|SetIsBraking false)))

(event Input|AxisEvents|InputAxisMoveRight
  (params (AxisValue :type Float%20%28single-precision%29))
  (bind _vehicleroot (Variables|Default|GetVehicleRoot))
  ;[1 1 1] Player Input
  ;;[1 1 1] Move Right/Left
  (Variables|State|SetDesiredLeftRight (Math|Float|Clamp(Float) (+ (* AxisValue (Variables|Gameplay|GetTurnSpeed) (Utilities|Time|GetWorldDeltaSeconds)) (Variables|State|GetDesiredLeftRight)) (Variables|Gameplay|GetLeftLaneLocalOffset) (Variables|Gameplay|GetRightLaneLocalOffset)))
  (Transformation|SetRelativeLocation (Variables|Default|GetVehicleRoot) (Math|Vector|MakeVector 0.0 (Variables|State|GetDesiredLeftRight) 0.0) false false)
  (Variables|State|SetIsTurning (!= (.y (Transformation|GetWorldLocation _vehicleroot)) (.y (Variables|State|GetPreviousLocation))))
  (Variables|State|SetPreviousLocation (Transformation|GetWorldLocation _vehicleroot)))

(fn ConstructionScript)

(fn EnoughTimeBetweenDrops
  (bind _returnvalue (Utilities|Time|GetTimeSeconds))
  (if (>= _returnvalue (+ (Variables|State|GetLastBrainDropTime) (Variables|Gameplay|GetMinTimeBetweenBrainDrops)))
    (Variables|State|SetLastBrainDropTime _returnvalue)
    (return true)
    (else
      (return false))))

(fn ComputeIsSlowingDown
  (bind _currentspeed (Variables|State|GetCurrentSpeed))
  (Variables|State|SetIsSlowingDown (Math|Boolean|ANDBoolean (Variables|State|GetIsBraking) (> _currentspeed (Variables|Gameplay|Braking|GetForwardSpeedWhenBraking)) (< _currentspeed (Variables|Gameplay|GetForwardSpeed))))
  (return))