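; BP_Zombie is a zombie that waits for a brain delivery and runs off with it once received.
; A looping timer compares its X position to the player's, flags the delivery as missed once the player passes a threshold, then stops.
; Receiving a brain turns it around and enables Tick, which is otherwise off, to move it forward at RunSpeed.
; DestroyZombie removes both the held brain and the zombie.
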(event Custom|OnReceivedBrain
  (params (Brain :type Actor%20Object%20Reference))
  (bind _returnvalue (Transformation|GetActorRotation))
  (Variables|State|SetBrainPackage Brain)
  (Variables|State|SetIsHoldingBrain true)
  (Actor|Tick|SetActorTickEnabled true)
  (Transformation|SetActorRotation (Math|Rotator|MakeRotator (.roll _returnvalue) (.pitch _returnvalue) (+ (.yaw _returnvalue) 1.8e+02))))

(event Custom|GetPositionRelationToPlayer
  (bind _returnvalue (Transformation|GetActorLocation))
  (bind _playerpawn (Variables|State|GetPlayerPawn))
  (bind _misseddeliverythreshold (Variables|Gameplay|GetMissedDeliveryThreshold))
  (bind _returnvalue_2 (Transformation|GetActorLocation _playerpawn))
  (bind _returnvalue_3 (+ (.x _returnvalue) _misseddeliverythreshold))
  (bind _returnvalue_4 (< _returnvalue_3 (.x _returnvalue_2)))
  (if _returnvalue_4
    (Variables|State|SetDeliveryWasMissed _returnvalue_4)
    (Utilities|Time|ClearandInvalidateTimerbyHandle (Variables|State|GetTimerHandle))))

(event Custom|DestroyZombie
  (bind _brainpackage (Variables|State|GetBrainPackage))
  (Utilities|IsValid _brainpackage
    (:Is%20Valid
      (Actor|DestroyActor _brainpackage))
    (:Is%20Not%20Valid
      _))
  (Actor|DestroyActor))

(event EventBeginPlay
  (Actor|Tick|SetActorTickEnabled false)
  (bind _output_get (Variables|State|SetPlayerPawn (Game|Player|GetPlayerPawn 0)))
  (Utilities|IsValid _output_get
    (:Is%20Valid
      (bind _returnvalue (Utilities|Time|SetTimerbyEvent (delegate Custom|GetPositionRelationToPlayer) 0.2 true))
      (Variables|State|SetTimerHandle _returnvalue))))

(event Collision|EventActorBeginOverlap
  (params (OtherActor :type Actor%20Object%20Reference)))

(event EventTick
  (params (DeltaSeconds :type Float%20%28single-precision%29))
  (Transformation|SetActorLocation (+ (Transformation|GetActorLocation) (* (Transformation|GetActorForwardVector) (* DeltaSeconds (Variables|Gameplay|GetRunSpeed)))) false false))

(fn ConstructionScript)

(fn NewFunction0)