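; BP_EndlessConfigSpawner builds an endless road of chained BP_RoadSegments and places BP_BrainDropZones on segments chosen by a BrainDeliverySpawnConfig.
; BeginPlay validates the config, then spawns warmup and starting segments, each at the previous one's attach point.
; NewSpawnRoadSegment adds drop zones at target segment numbers, and the config repeats, offset by its last segment number each pass.
; An older RoadSegmentSpawnConfig path with vehicle spawns remains but is disconnected.
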(event Custom|SpawnRoadSegment
  (bind _self self)
  (bind _spawnconfigindex (Variables|State|GetSpawnConfigIndex))
  (bind _currentspawnconfig (Variables|State|GetCurrentSpawnConfig))
  (bind _spawnconfig (Variables|/Game/Game/Blueprints/RoadSegmentSpawnConfigs/BP_RoadSegmentSpawnConfigBase.BP_RoadSegmentSpawnConfigBase_C|GetSpawnConfig _currentspawnconfig))
  (bind _output (Utilities|Array|Get(acopy) _spawnconfig _spawnconfigindex))
  ;[1 1 1] Spawn next segment of road
  (if (== (Variables|State|GetNextTargetRoadSegment) (Variables|State|GetRoadSegmentNumber))
    (bind _returnvalue (Game|SpawnActorfromClass "/Game/Game/Blueprints/BP_RoadSegment.BP_RoadSegment_C" (Variables|State|GetNextSpawnTransform) "Undefined" 0 _self (Utilities|Struct|MakeSBP_RoadSegmentConfig (Variables|State|GetRoadSegmentNumber) (.braindelivery _output) (.vehiclespawns _output)) false 0 0 0))
    (Utilities|IsValid _returnvalue
      (:Is%20Valid
        (bind _nextsegmentattachpoint (Default|GetNextSegmentAttachPoint _returnvalue))
        (Variables|State|SetNextSpawnTransform _nextsegmentattachpoint))
      (:Is%20Not%20Valid
        _))
    (Math|Integer|IncrementInt (Variables|State|GetRoadSegmentNumber)
      (:%20%20
        (CallFunction|SetNextTargetRoadSegment)))
    (else
      (bind _returnvalue_2 (Game|SpawnActorfromClass "/Game/Game/Blueprints/BP_RoadSegment.BP_RoadSegment_C" (Variables|State|GetNextSpawnTransform) "Undefined" 0 _self (Utilities|Struct|MakeSBP_RoadSegmentConfig (Variables|State|GetRoadSegmentNumber) "NewEnumerator0" "(INVALID)") false 0 0 0))
      (Utilities|IsValid _returnvalue_2
        (:Is%20Valid
          (bind _nextsegmentattachpoint_2 (Default|GetNextSegmentAttachPoint _returnvalue_2))
          (Variables|State|SetNextSpawnTransform _nextsegmentattachpoint_2))
        (:Is%20Not%20Valid
          _))
      (Math|Integer|IncrementInt (Variables|State|GetRoadSegmentNumber)))))

(event Custom|SpawnWarmupRoad
  (for _index (range 1 (Variables|Gameplay|GetWarmupRoadSegments))
    (bind _returnvalue (Game|SpawnActorfromClass :Class "/Game/Game/Blueprints/BP_RoadSegment.BP_RoadSegment_C" :SpawnTransform (Variables|State|GetNextSpawnTransform) :CollisionHandlingOverride "Undefined" :RoadSpawnSystem 0 :IsWarmupRoad true :EndlessConfigSpawner 0 :Instigator 0))
    (Utilities|IsValid _returnvalue
      (:Is%20Valid
        (bind _nextsegmentattachpoint (Default|GetNextSegmentAttachPoint _returnvalue))
        (Variables|State|SetNextSpawnTransform _nextsegmentattachpoint)))))

(event Custom|SetIterationOffset
  (bind _currentbraindeliveryconfig (Variables|State|GetCurrentBrainDeliveryConfig))
  (bind _braindeliveryconfig (Variables|/Game/Game/Blueprints/BrainDeliverySpawnConfigs/BP_BrainDeliveryConfigBase.BP_BrainDeliveryConfigBase_C|GetBrainDeliveryConfig _currentbraindeliveryconfig))
  ;[1 1 1] Set config iteration offset, evey time through the config this will be base number to calculate NextTargetRoadSegment
  (Variables|State|SetIterationOffset (.roadsegmentnumber (Utilities|Array|Get(acopy) _braindeliveryconfig (- (Utilities|Array|Length _braindeliveryconfig) 1)))))

(event Custom|SetInitialNextTargetRoadSegment
  ;[1 1 1] Initial Target RoadSegment is first entry in RoadSegmentSpawnConfig
  (Variables|State|SetNextTargetRoadSegment (.roadsegmentnumber (Utilities|Array|Get(acopy) (Variables|/Game/Game/Blueprints/BrainDeliverySpawnConfigs/BP_BrainDeliveryConfigBase.BP_BrainDeliveryConfigBase_C|GetBrainDeliveryConfig (Variables|State|GetCurrentBrainDeliveryConfig))))))

(event Custom|SpawnStartingRoadSegments
  ;[1 1 1] Spawn StartingRoadSegments of road
  (if (<= (Variables|Gameplay|GetStartingRoadSegments) 0)
    (Variables|Gameplay|SetStartingRoadSegments 1))
  (for _index (range 0 (Variables|Gameplay|GetStartingRoadSegments))
    (CallFunction|NewSpawnRoadSegment)))

(event Custom|SetNextTargetRoadSegment
  ;[1 1 1] Comment
  (bind _result (Math|Integer|IncrementInt (Variables|State|GetSpawnConfigIndex))
    (:%20%20
      (if (>= _result (Utilities|Array|Length (Variables|/Game/Game/Blueprints/BrainDeliverySpawnConfigs/BP_BrainDeliveryConfigBase.BP_BrainDeliveryConfigBase_C|GetBrainDeliveryConfig (Variables|State|GetCurrentBrainDeliveryConfig))))
        (Variables|State|SetSpawnConfigIndex 0)
        (Math|Integer|IncrementInt (Variables|State|GetTimesThroughConfig)
          (:%20%20
            _)))
      (if (== (+ (* (Variables|State|GetIterationOffset) (Variables|State|GetTimesThroughConfig)) (.roadsegmentnumber (Utilities|Array|Get(acopy) (Variables|/Game/Game/Blueprints/BrainDeliverySpawnConfigs/BP_BrainDeliveryConfigBase.BP_BrainDeliveryConfigBase_C|GetBrainDeliveryConfig (Variables|State|GetCurrentBrainDeliveryConfig)) (Variables|State|GetSpawnConfigIndex)))) (Variables|State|GetNextTargetRoadSegment))
        (Variables|State|SetNextTargetRoadSegment (+ (+ (* (Variables|State|GetIterationOffset) (Variables|State|GetTimesThroughConfig)) (.roadsegmentnumber (Utilities|Array|Get(acopy) (Variables|/Game/Game/Blueprints/BrainDeliverySpawnConfigs/BP_BrainDeliveryConfigBase.BP_BrainDeliveryConfigBase_C|GetBrainDeliveryConfig (Variables|State|GetCurrentBrainDeliveryConfig)) (Variables|State|GetSpawnConfigIndex)))) 1))
        (else
          (Variables|State|SetNextTargetRoadSegment (+ (* (Variables|State|GetIterationOffset) (Variables|State|GetTimesThroughConfig)) (.roadsegmentnumber (Utilities|Array|Get(acopy) (Variables|/Game/Game/Blueprints/BrainDeliverySpawnConfigs/BP_BrainDeliveryConfigBase.BP_BrainDeliveryConfigBase_C|GetBrainDeliveryConfig (Variables|State|GetCurrentBrainDeliveryConfig)) (Variables|State|GetSpawnConfigIndex))))))))))

(event Custom|SetBrainDeliveryIterationOffset
  (bind _currentbraindeliveryconfig (Variables|State|GetCurrentBrainDeliveryConfig))
  (bind _braindeliveryconfig (Variables|/Game/Game/Blueprints/BrainDeliverySpawnConfigs/BP_BrainDeliveryConfigBase.BP_BrainDeliveryConfigBase_C|GetBrainDeliveryConfig _currentbraindeliveryconfig))
  (Variables|State|SetIterationOffset (.roadsegmentnumber (Utilities|Array|Get(acopy) _braindeliveryconfig (- (Utilities|Array|Length _braindeliveryconfig) 1)))))

(event Custom|NewSpawnRoadSegment
  (bind _self self)
  (bind _spawnconfigindex (Variables|State|GetSpawnConfigIndex))
  (bind _currentbraindeliveryconfig (Variables|State|GetCurrentBrainDeliveryConfig))
  (bind _roadsegmentnumber (Variables|State|GetRoadSegmentNumber))
  (bind _braindeliveryconfig (Variables|/Game/Game/Blueprints/BrainDeliverySpawnConfigs/BP_BrainDeliveryConfigBase.BP_BrainDeliveryConfigBase_C|GetBrainDeliveryConfig _currentbraindeliveryconfig))
  (bind _output (Utilities|Array|Get(acopy) _braindeliveryconfig _spawnconfigindex))
  (if (== (Variables|State|GetNextTargetRoadSegment) (Variables|State|GetRoadSegmentNumber))
    (bind _returnvalue (Game|SpawnActorfromClass :Class "/Game/Game/Blueprints/BP_RoadSegment.BP_RoadSegment_C" :SpawnTransform (Variables|State|GetNextSpawnTransform) :CollisionHandlingOverride "Undefined" :RoadSpawnSystem 0 :RoadSegmentNumber _roadsegmentnumber :EndlessConfigSpawner _self :Instigator 0))
    (Utilities|IsValid _returnvalue
      (:Is%20Valid
        (bind _nextsegmentattachpoint (Default|GetNextSegmentAttachPoint _returnvalue))
        (Variables|State|SetNextSpawnTransform _nextsegmentattachpoint)
        (bind _deliverytransform (Default|GetBrainDeliveryTransform _returnvalue (.braindelivery _output)))
        (Game|SpawnActorfromClass "/Game/Game/Blueprints/BP_BrainDropZone.BP_BrainDropZone_C" _deliverytransform "Undefined" 0 (.braindelivery _output) 0)
        (Math|Integer|IncrementInt (Variables|State|GetRoadSegmentNumber)
          (:%20%20
            (CallFunction|SetNextTargetRoadSegment)))))
    (else
      (bind _returnvalue_2 (Game|SpawnActorfromClass :Class "/Game/Game/Blueprints/BP_RoadSegment.BP_RoadSegment_C" :SpawnTransform (Variables|State|GetNextSpawnTransform) :CollisionHandlingOverride "Undefined" :RoadSpawnSystem 0 :RoadSegmentNumber _roadsegmentnumber :EndlessConfigSpawner _self :Instigator 0))
      (Utilities|IsValid _returnvalue_2
        (:Is%20Valid
          (bind _nextsegmentattachpoint_2 (Default|GetNextSegmentAttachPoint _returnvalue_2))
          (Variables|State|SetNextSpawnTransform _nextsegmentattachpoint_2))
        (:Is%20Not%20Valid
          _))
      (Math|Integer|IncrementInt (Variables|State|GetRoadSegmentNumber)))))

(event EventBeginPlay
  (bind _returnvalue (Game|ConstructObjectfromClass (Variables|Gameplay|GetBrainDeliverySpawnConfig) self))
  (Variables|State|SetCurrentBrainDeliveryConfig _returnvalue)
  (bind _result (CallFunction|VerifyBrainDeliverySetup))
  (if _result
    (CallFunction|SetBrainDeliveryIterationOffset)
    (CallFunction|SetInitialNextTargetRoadSegment)
    (CallFunction|SpawnWarmupRoad)
    (CallFunction|SpawnStartingRoadSegments)
    (else
      (Development|PrintString "Error: BP_EndlessConfigSpawn will not spawn any road segments, see previous error" true true "(R=1.000000,G=0.000000,B=0.000000,A=1.000000)"))))

(fn ConstructionScript)

(fn VerifySetup
  ;[1 1 1] Check RoadSegmentConfig has at least 1 entry
  (if (> (Utilities|Array|Length (Variables|/Game/Game/Blueprints/RoadSegmentSpawnConfigs/BP_RoadSegmentSpawnConfigBase.BP_RoadSegmentSpawnConfigBase_C|GetSpawnConfig (Variables|State|GetCurrentSpawnConfig))) 0)
    ;[1 1 1] Verify RoadSegmentNumber in RoadSegmentSpawnConfig are in increasing order
    (for (_array_element _array_index) (Variables|/Game/Game/Blueprints/RoadSegmentSpawnConfigs/BP_RoadSegmentSpawnConfigBase.BP_RoadSegmentSpawnConfigBase_C|GetSpawnConfig (Variables|State|GetCurrentSpawnConfig))
      (if (== _array_index 0)
        (LocalVariables|SetPreviousRoadSegmentNumber (.roadsegmentnumber _array_element))
        (elif (<= (.roadsegmentnumber _array_element) (LocalVariables|GetPreviousRoadSegmentNumber))
          (Development|PrintString (Utilities|String|Append "Error: BP_RoadSpawnSystem, RoadSegmentSpawnConfig.RoadSegmentNumber at index  " (Utilities|String|ToString(Integer) _array_index) " is less than previous index") true true "(R=1.000000,G=0.000000,B=0.000000,A=1.000000)" 1e+01)
          (return false))))
    (return true)
    (else
      (Development|PrintString "Error: RoadSegmentSpawnConfig has no entries!" true true "(R=1.000000,G=0.000000,B=0.000000,A=1.000000)" 1e+01)
      (return false))))

(fn MakeNextRoadSegmentConfig
  (params (RoadSegmentConfig :type SBP%20Road%20Segment%20Config%20Structure))
  (return (Utilities|Struct|MakeSBP_RoadSegmentConfig (Variables|State|GetRoadSegmentNumber) (.braindelivery RoadSegmentConfig) (.vehiclespawns RoadSegmentConfig))))

(fn VerifyBrainDeliverySetup
  (Utilities|FlowControl|Sequence
    (:then_0
      (if (not (> (Utilities|Array|Length (Variables|/Game/Game/Blueprints/BrainDeliverySpawnConfigs/BP_BrainDeliveryConfigBase.BP_BrainDeliveryConfigBase_C|GetBrainDeliveryConfig (Variables|State|GetCurrentBrainDeliveryConfig))) 0))
        (Development|PrintString "Error: BrainDeliveryConfig has no entries!" true true "(R=1.000000,G=0.000000,B=0.000000,A=1.000000)" 1e+01)
        (return false)))
    (:then_1
      (if (not (> (.roadsegmentnumber (Utilities|Array|Get(acopy) (Variables|/Game/Game/Blueprints/BrainDeliverySpawnConfigs/BP_BrainDeliveryConfigBase.BP_BrainDeliveryConfigBase_C|GetBrainDeliveryConfig (Variables|State|GetCurrentBrainDeliveryConfig)))) 0))
        (Development|PrintString "Error: BrainDeliveryConfig, first RoadSegmentNumber must be greater than 0!" true true "(R=1.000000,G=0.000000,B=0.000000,A=1.000000)" 1e+01)
        (return false)))
    (:then_2
      (for (_array_element _array_index) (Variables|/Game/Game/Blueprints/BrainDeliverySpawnConfigs/BP_BrainDeliveryConfigBase.BP_BrainDeliveryConfigBase_C|GetBrainDeliveryConfig (Variables|State|GetCurrentBrainDeliveryConfig))
        (if (== _array_index 0)
          (LocalVariables|SetPreviousRoadSegmentNumber 0)
          (elif (<= (.roadsegmentnumber _array_element) (LocalVariables|GetPreviousRoadSegmentNumber))
            (Development|PrintString (Utilities|String|Append "Error: BP_EndlessConfigSpawn, BrainDeliverySpawnConfig.RoadSegmentNumber at index  " (Utilities|String|ToString(Integer) _array_index) " is less than previous index"))
            (return false))))
      (return true))))