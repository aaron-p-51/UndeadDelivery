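; BP_HealthComponent is a health component that tracks current health and grants temporary invincibility after damage.
; Health starts at the default on BeginPlay, and LoseHealth subtracts a clamped amount unless invincibility blocks it.
; Each accepted hit starts a timer that ends invincibility, with dispatchers broadcasting health and invincibility changes.
; LoseHealth also compares game time against LastTimeHealthLost, which this graph never updates.
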(event Custom|LoseHealth
  (params (Amount :type Integer))
  (if (and (not (Variables|State|GetInvincibleAfterHealthLoss)) (>= (Utilities|Time|GetTimeSeconds) (+ (Variables|State|GetLastTimeHealthLost) (Variables|GamePlay|GetHealthLossInvincibilityTime))))
    (bind _output_get (Variables|State|SetCurrentHealth (Math|Integer|Clamp(Integer) (- (Variables|State|GetCurrentHealth) Amount) 0 (Variables|GamePlay|GetDefaultHealth))))
    (Default|CallOnHealthValueChanged _output_get)
    (bind _output_get_2 (Variables|State|SetInvincibleAfterHealthLoss true))
    (Default|CallInvincibilityChange _output_get_2)
    (Utilities|Time|SetTimerbyEvent (delegate Custom|EndInvincibility) (Variables|GamePlay|GetHealthLossInvincibilityTime))))

(event Custom|EndInvincibility
  (bind _output_get (Variables|State|SetInvincibleAfterHealthLoss false))
  (Default|CallInvincibilityChange _output_get))

(event EventBeginPlay
  (bind _output_get (Variables|State|SetCurrentHealth (Variables|GamePlay|GetDefaultHealth)))
  (Default|CallOnHealthValueChanged _output_get))

(event EventTick
  (params (DeltaSeconds :type Float%20%28single-precision%29)))

(fn GetCurrentHealth
  (return (Variables|State|GetCurrentHealth)))