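; Actor component that manages a limited brake resource the player spends while braking and regains afterward.
; A state enum (Charged, Braking, Depleted, RechargeDelay, Recharging) drives Tick, which drains or refills the current amount at set rates.
; Start and stop input events switch states, using a cancellable timer to delay recharge after release.
; IsBraking exposes whether braking is active.
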(event Custom|UseBrakeAmount
  (params (DeltaSeconds :type Float%20%28single-precision%29))
  ;[1 1 1] Use available brake amount
  (if (> (Variables|State|GetCurrentBrakeAmount) 0.0)
    (bind _output_get (Variables|State|SetCurrentBrakeAmount (- (Variables|State|GetCurrentBrakeAmount) (* (Variables|Gameplay|GetUseBrakeRate) DeltaSeconds))))
    (if (<= _output_get 0.0)
      (Variables|State|SetBrakeState "NewEnumerator4"))))

(event Custom|RechargeBrakeAmount
  (params (DeltaSeconds :type Float%20%28single-precision%29))
  ;[1 1 1] Recharge available brake amount
  (if (< (Variables|State|GetCurrentBrakeAmount) (Variables|Gameplay|GetDefaultBrakeAmount))
    (bind _output_get (Variables|State|SetCurrentBrakeAmount (+ (Variables|State|GetCurrentBrakeAmount) (* (Variables|Gameplay|GetBrakeRechargeRate) DeltaSeconds))))
    (if (>= _output_get (Variables|Gameplay|GetDefaultBrakeAmount))
      (Variables|State|SetBrakeState "NewEnumerator0"))))

(event Custom|StartUseBrake
  ;[1 1 1] Input, player using brake
  (if (> (Variables|State|GetCurrentBrakeAmount) 0.0)
    (Variables|State|SetBrakeState "NewEnumerator1")
    (Utilities|Time|ClearandInvalidateTimerbyHandle (Variables|Default|GetTimerHandle))))

(event Custom|StopUseBrake
  (bind _brakerechargedelay (Variables|Gameplay|GetBrakeRechargeDelay))
  ;[1 1 1] Input, player stop using brake
  (if (< (Variables|State|GetCurrentBrakeAmount) (Variables|Gameplay|GetDefaultBrakeAmount))
    (if (> _brakerechargedelay 0.0)
      (Variables|State|SetBrakeState "NewEnumerator2")
      (bind _returnvalue (Utilities|Time|SetTimerbyEvent (delegate Custom|OnBrakeRechargeDelayComplete) _brakerechargedelay))
      (Variables|Default|SetTimerHandle _returnvalue)
      (else
        (CallFunction|HandleonBrakeRechargeDelayComplete)))))

(event Custom|OnBrakeRechargeDelayComplete
  ;[1 1 1] Input, player stop using brake
  (CallFunction|HandleonBrakeRechargeDelayComplete))

(event Custom|HandleOnBrakeRechargeDelayComplete
  ;[1 1 1] Input, player stop using brake
  (Variables|State|SetBrakeState "NewEnumerator3"))

(event EventBeginPlay
  (Variables|State|SetCurrentBrakeAmount (Variables|Gameplay|GetDefaultBrakeAmount))
  (Variables|State|SetBrakeState "NewEnumerator0"))

(event EventTick
  (params (DeltaSeconds :type Float%20%28single-precision%29))
  (switch Utilities|FlowControl|Switch|SwitchonEBP_BrakeState (Variables|State|GetBrakeState)
    (:NewEnumerator1
      (CallFunction|UseBrakeAmount DeltaSeconds))
    (:NewEnumerator3
      (CallFunction|RechargeBrakeAmount DeltaSeconds))))

(fn IsBraking
  (return (Utilities|Enum|Equal(Enum) (Variables|State|GetBrakeState) "NewEnumerator1")))