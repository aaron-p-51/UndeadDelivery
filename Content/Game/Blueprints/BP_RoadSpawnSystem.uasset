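; Road spawner that builds a chain of BP_RoadSegment actors, each placed at the previous segment's attach point and given a reference back to the spawner.
; BeginPlay validates that the spawn config is non-empty and ascending by segment number, then spawns the starting segments.
; Segments matching a target number take that entry's brain delivery and vehicle spawns.
; The config repeats indefinitely, offset each pass by its last entry's segment number.
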(event Custom|SpawnRoadSegment
  (bind _roadsegmentnumber (Variables|State|GetRoadSegmentNumber))
  (bind _nexttargetroadsegment (Variables|State|GetNextTargetRoadSegment))
  (bind _returnvalue (== _nexttargetroadsegment _roadsegmentnumber))
  ;[1 1 1] Spawn next segment of road
  (if _returnvalue
    (CallFunction|MakeNextRoadSegmentConfig (Utilities|Array|Get(acopy) (Variables|Gameplay|GetRoadSegmentSpawnConfig) (Variables|State|GetSpawnConfigIndex)))
    (else
      (bind _nextroadsegmentconfig (CallFunction|MakeNextRoadSegmentConfig))))
  (bind _returnvalue_2 (Game|SpawnActorfromClass "/Game/Game/Blueprints/BP_RoadSegment.BP_RoadSegment_C" (Variables|State|GetNextSpawnTransform) "Undefined" 0 self 0 "NewEnumerator1" _nextroadsegmentconfig 0))
  (Math|Integer|IncrementInt (Variables|State|GetRoadSegmentNumber)
    (:%20%20
      (Utilities|IsValid _returnvalue_2
        (:Is%20Valid
          (bind _nextsegmentattachpoint (Default|GetNextSegmentAttachPoint _returnvalue_2))
          (Variables|State|SetNextSpawnTransform _nextsegmentattachpoint))
        (:Is%20Not%20Valid
          _))
      (if _returnvalue
        (CallFunction|SetNextTargetRoadSegment)))))

(event Custom|SetIterationOffset
  (bind _roadsegmentspawnconfig (Variables|Gameplay|GetRoadSegmentSpawnConfig))
  ;[1 1 1] Set config iteration offset, evey time through the config this will be base number to calculate NextTargetRoadSegment
  (Variables|State|SetIterationOffset (.roadsegmentnumber (Utilities|Array|Get(acopy) _roadsegmentspawnconfig (- (Utilities|Array|Length _roadsegmentspawnconfig) 1)))))

(event Custom|SetInitialNextTargetRoadSegment
  ;[1 1 1] Initial Target RoadSegment is first entry in RoadSegmentSpawnConfig
  (Variables|State|SetNextTargetRoadSegment (.roadsegmentnumber (Utilities|Array|Get(acopy) (Variables|Gameplay|GetRoadSegmentSpawnConfig)))))

(event Custom|SpawnStartingRoadSegments
  ;[1 1 1] Spawn StartingRoadSegments of road
  (for _index (range 0 (Math|Integer|Absolute(Integer) (Variables|Gameplay|GetStartingRoadSegments)))
    (CallFunction|SpawnRoadSegment)))

(event Custom|SetNextTargetRoadSegment
  ;[1 1 1] Comment
  (bind _result (Math|Integer|IncrementInt (Variables|State|GetSpawnConfigIndex))
    (:%20%20
      (if (>= _result (Utilities|Array|Length (Variables|Gameplay|GetRoadSegmentSpawnConfig)))
        (Variables|State|SetSpawnConfigIndex 0)
        (Math|Integer|IncrementInt (Variables|State|GetTimesThroughConfig)
          (:%20%20
            _)))
      (bind _output_get (Variables|State|SetNextTargetRoadSegment (+ (* (Variables|State|GetIterationOffset) (Variables|State|GetTimesThroughConfig)) (.roadsegmentnumber (Utilities|Array|Get(acopy) (Variables|Gameplay|GetRoadSegmentSpawnConfig) (Variables|State|GetSpawnConfigIndex))))))
      (Development|PrintString (Utilities|String|ToString(Integer) _output_get) true true "(R=0.000000,G=0.660000,B=1.000000,A=1.000000)" 1e+02))))

(event EventBeginPlay
  (bind _setupproperly (CallFunction|VerifySetup))
  (if _setupproperly
    (CallFunction|SetIterationOffset)
    (CallFunction|SetInitialNextTargetRoadSegment)
    (CallFunction|SpawnStartingRoadSegments)
    (else
      (Development|PrintString "Error: RoadSpawnSystem will not spawn any road segments, see previous error" true true "(R=1.000000,G=0.000000,B=0.000000,A=1.000000)"))))

(fn ConstructionScript)

(fn VerifySetup
  ;[1 1 1] Check RoadSegmentConfig has at least 1 entry
  (if (> (Utilities|Array|Length (Variables|Gameplay|GetRoadSegmentSpawnConfig)) 0)
    ;[1 1 1] Verify RoadSegmentNumber in RoadSegmentSpawnConfig are in increasing order
    (for (_array_element _array_index) (Variables|Gameplay|GetRoadSegmentSpawnConfig)
      (if (== _array_index 0)
        (LocalVariables|SetPreviousRoadSegmentNumber (.roadsegmentnumber _array_element))
        (elif (<= (.roadsegmentnumber _array_element) (LocalVariables|GetPreviousRoadSegmentNumber))
          (Development|PrintString (Utilities|String|Append "Error: BP_RoadSpawnSystem, RoadSegmentSpawnConfig.RoadSegmentNumber at index  " (Utilities|String|ToString(Integer) _array_index) " is less than previous index") true true "(R=1.000000,G=0.000000,B=0.000000,A=1.000000)" 1e+01)
          (return false))))
    (return true)
    (else
      (Development|PrintString "Error: RoadSegmentSpawnConfig has no entries!" true true "(R=1.000000,G=0.000000,B=0.000000,A=1.000000)" 1e+01)
      (return false))))

(fn MakeNextRoadSegmentConfig
  (params (RoadSegmentConfig :type SBP%20Road%20Segment%20Config%20Structure))
  (return (Utilities|Struct|MakeSBP_RoadSegmentConfig (Variables|State|GetRoadSegmentNumber) (.braindelivery RoadSegmentConfig) (.vehiclespawns RoadSegmentConfig))))