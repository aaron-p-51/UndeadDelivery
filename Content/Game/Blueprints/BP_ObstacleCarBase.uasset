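; Base Blueprint for obstacle cars that drive forward at a constant speed, moved each Tick without sweep.
; A looping timer destroys the car once it falls far enough behind the player pawn along world X.
; A spawn check event destroys the car if it overlaps another obstacle car, then disables the check's collision; its only call in this graph is disconnected.
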(event Custom|CheckIfBehindPlayerPawn
  ;[1 1 1] Destroy this obstical car if sufficiently behind player pawn
  (if (< (+ (.x (Transformation|GetActorLocation)) (Variables|Gameplay|GetBehindPlayerThreshold)) (.x (Transformation|GetActorLocation (Variables|State|GetPlayerPawn))))
    (Actor|DestroyActor)))

(event Custom|CheckForCollisionOnSpawn
  (for _array_element (Collision|GetOverlappingActors (Variables|Default|GetSpawnCheckOverlap) "BP_ObstacleCarBase_C" :!class /Script/Engine.PrimitiveComponent)
    (if (!= _array_element self)
      (Actor|DestroyActor)))
  (Collision|SetCollisionEnabled (Variables|Default|GetSpawnCheckOverlap) "NoCollision"))

(event EventBeginPlay
  (Variables|State|SetPlayerPawn (Game|Player|GetPlayerPawn 0))
  (Utilities|Time|SetTimerbyEvent (delegate Custom|CheckIfBehindPlayerPawn) (Variables|Gameplay|GetCheckDestroyInterval) true))

(event EventTick
  (params (DeltaSeconds :type Float%20%28single-precision%29))
  ;[1 1 1] Move forward at constant speed
  (Transformation|SetActorLocation (+ (Transformation|GetActorLocation) (* (Transformation|GetActorForwardVector) (* DeltaSeconds (Variables|State|GetForwardSpeed)))) false false))

(fn ConstructionScript)