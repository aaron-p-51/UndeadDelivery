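; BP_BrainDropZone is a brain drop zone actor that spawns and owns a BP_Zombie when play begins.
; The BrainDelivery setting selects whether the zombie spawns at the left or right pickup spawn location component.
; The spawned zombie is stored in a variable and exposed through GetZombie.
; No overlap or drop handling lives in this Blueprint, as the overlap and tick events are empty.
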(event EventBeginPlay
  (switch Utilities|FlowControl|Switch|SwitchonEBP_BrainDelivery (Variables|State|GetBrainDelivery)
    (:NewEnumerator1
      (bind _returnvalue (Game|SpawnActorfromClass "/Game/Game/Blueprints/BP_Zombie.BP_Zombie_C" (Transformation|GetWorldTransform (Variables|Default|GetLeftPickupZombieSpawnLocation)) "Undefined" 0 0))
      (Variables|State|SetZombie _returnvalue))
    (:NewEnumerator2
      (bind _returnvalue_2 (Game|SpawnActorfromClass "/Game/Game/Blueprints/BP_Zombie.BP_Zombie_C" (Transformation|GetWorldTransform (Variables|Default|GetRightPickupZombieSpawnLocation)) "Undefined" 0 0))
      (Variables|State|SetZombie _returnvalue_2))))

(event Collision|EventActorBeginOverlap
  (params (OtherActor :type Actor%20Object%20Reference)))

(event EventTick
  (params (DeltaSeconds :type Float%20%28single-precision%29)))

(fn ConstructionScript)

(fn GetZombie
  (return (Variables|State|GetZombie)))